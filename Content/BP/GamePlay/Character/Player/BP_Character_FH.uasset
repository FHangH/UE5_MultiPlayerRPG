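; Player character Blueprint that tints its Manny mesh with a selectable player color.
; FHUpdateCharacterColor calls ChangeColor, which maps the chosen color option to a Color value through a switch.
; It then creates dynamic material instances on both mesh slots and sets their MyColor parameter.
; OnRep_Color repeats the material update when the replicated Color arrives, keeping the tint in sync across the network.
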(event `self.FH_UpdateCharacterColor`
  (params (Color :type "EFH_Color Enum" :default "EFHC_WHITE"))
  (`self.ChangeColor` Color))

(fn `ChangeColor`
  (params (Selection :type "EFH_Color Enum" :default "EFHC_WHITE"))
  (`self.SwicthPlayerColor` Selection)
  (bind _returnvalue (`PrimitiveComponent.CreateDynamicMaterialInstance` (`self.Mesh`) 0 "/Game/Assets/UE5_Character/Mannequins/Materials/Instances/Manny/MI_Manny_02.MI_Manny_02" "None"))
  (`MaterialInstanceDynamic.SetVectorParameterValue` _returnvalue "MyColor" (`self.Color`))
  (bind _returnvalue_2 (`PrimitiveComponent.CreateDynamicMaterialInstance` (`self.Mesh`) 1 "/Game/Assets/UE5_Character/Mannequins/Materials/Instances/Manny/MI_Manny_01.MI_Manny_01" "None"))
  (`MaterialInstanceDynamic.SetVectorParameterValue` _returnvalue_2 "MyColor" (`self.Color`)))

(fn `OnRep_Color`
  (bind _returnvalue (`PrimitiveComponent.CreateDynamicMaterialInstance` (`self.Mesh`) 0 "/Game/Assets/UE5_Character/Mannequins/Materials/Instances/Manny/MI_Manny_02.MI_Manny_02" "None"))
  (`MaterialInstanceDynamic.SetVectorParameterValue` _returnvalue "MyColor" (`self.Color`))
  (bind _returnvalue_2 (`PrimitiveComponent.CreateDynamicMaterialInstance` (`self.Mesh`) 1 "/Game/Assets/UE5_Character/Mannequins/Materials/Instances/Manny/MI_Manny_01.MI_Manny_01" "None"))
  (`MaterialInstanceDynamic.SetVectorParameterValue` _returnvalue_2 "MyColor" (`self.Color`)))

(fn `UserConstructionScript`)